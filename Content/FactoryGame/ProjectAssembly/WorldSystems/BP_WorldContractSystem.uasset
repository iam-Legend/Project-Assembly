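; BP_WorldContractSystem is a world system that holds the library of Project Assembly contracts, currently filled with hardcoded test entries carrying cost, payout, state flags and image.
; On BeginPlay, SetContracts adds each entry whose ID is not already stored, using a parallel ID array for faster duplicate checks.
; ResetContracts overwrites both arrays with single placeholder values, then runs SetContracts again to repopulate them.
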(event `self.ReceiveBeginPlay`
  (`self.SetContracts`))

(fn `ResetContracts`
  (set `self.ContractsLib` (`|MakeArray` (struct) :!type "/Game/FactoryGame/ProjectAssembly/WorldSystems/PA_Contract Structure"))
  (set `self.ContractsLib_IDs` (`|MakeArray` "None" :!type "Name"))
  (`self.SetContracts`)
  (return))

(fn `SetContracts`
  (bind _contractslib_ids (`self.ContractsLib_IDs`))
  (for _array_element (`|MakeArray` (make `/Game/FactoryGame/ProjectAssembly/WorldSystems/PA_Contract` "1" "Test Contract #1" 500000 700000 true false true 0 false true "/Game/FactoryGame/ProjectAssembly/Textures/Icons/PA_ContractIcons/Beryl_Nut.Beryl_Nut") (make `/Game/FactoryGame/ProjectAssembly/WorldSystems/PA_Contract` "2" "Test Contract #2" 500000 1000000 true false false 0 false false "/Game/FactoryGame/ProjectAssembly/Textures/Icons/PA_ContractIcons/Beryl_Nut.Beryl_Nut") (make `/Game/FactoryGame/ProjectAssembly/WorldSystems/PA_Contract` "3" "Test Contract #3" 1000000 1200000 true false false 0 false false "/Game/FactoryGame/ProjectAssembly/Textures/Icons/PA_ContractIcons/Beryl_Nut.Beryl_Nut"))
    (bind _contractid (break `/Game/FactoryGame/ProjectAssembly/WorldSystems/PA_Contract` _array_element))
    (if (not (`KismetArrayLibrary.Array_Contains` _contractslib_ids _contractid))
      (`KismetArrayLibrary.Array_Add` _contractslib_ids _contractid)
      (`KismetArrayLibrary.Array_Add` (`self.ContractsLib`) _array_element)))
  (return))

(fn `UserConstructionScript`)